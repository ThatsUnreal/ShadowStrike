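; SwordBP is a sword weapon actor whose visibility and wraith-mode effects can be toggled.
; ToggleVisibility hides or shows the root component and propagates the change to all its children.
; ToggleVFX sets the skeletal mesh's first material slot and drives the fire particle effect through its VertSurfaceActor parameter, passing the sword itself to show and clearing it to hide.
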(event `self.ReceiveBeginPlay`)

(event `/Game/_ShadowStrike/Blueprints/BPI_Weapons.ToggleVisibility`
  (params (`Hide?` :type Boolean))
  (if `Hide?`
    (`SceneComponent.SetVisibility` (`self.DefaultSceneRoot`) false true)
    (else
      (`SceneComponent.SetVisibility` (`self.DefaultSceneRoot`) true true))))

(fn `Toggle VFX`
  (params (`Show?` :type Boolean))
  (if `Show?`
    ;[1 1 1] Update the material of the wepaon when warith mode and toggle the fire particle effect
    (`FXSystemComponent.SetActorParameter` (`self.ParticleSystem`) "VertSurfaceActor" self)
    (`PrimitiveComponent.SetMaterial` (`self.SkeletalMesh`) 0 null)
    (else
      (`FXSystemComponent.SetActorParameter` (`self.ParticleSystem`) "VertSurfaceActor" null)
      (`PrimitiveComponent.SetMaterial` (`self.SkeletalMesh`) 0 null))))

(fn `UserConstructionScript`)