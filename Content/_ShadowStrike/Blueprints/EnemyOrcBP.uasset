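; EnemyOrcBP is a sword-wielding orc enemy that can be targeted while alive and shows a toggleable target indicator.
; It exposes events and functions for playing montages, setting and querying death state, and retrieving its mesh, with bow hand location stubbed to zero.
; Death activation turns off custom depth, ragdolls the mesh and detaches the sword as a physics object, separately from setting the Died flag.
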(event `/Game/_ShadowStrike/Blueprints/BPI_Character.PlayCharacterAnimMontage`
  (params (MontageToPlay :type "AnimMontage Object Reference"))
  ;[0.3543 1 0.8079] Montage play by interface function
  (`AnimInstance.Montage_Play` (`SkeletalMeshComponent.GetAnimInstance` (`self.Mesh`)) MontageToPlay 1.0 "MontageLength" 0.0 true))

(event `/Game/_ShadowStrike/Blueprints/BPI_Character.ActivateDeath`
  (bind _sword (`self.Sword`))
  (bind _mesh (`self.Mesh`))
  ;[1 0.1782 0.5955] Update character mesh properties and make the character go ragdoll & enable physics on holding weapon
  (`PrimitiveComponent.SetRenderCustomDepth` _mesh false)
  (`PrimitiveComponent.SetCollisionProfileName` _mesh "Ragdoll" true)
  (`PrimitiveComponent.SetSimulatePhysics` _mesh true)
  (`PrimitiveComponent.SetRenderCustomDepth` _sword false)
  (`PrimitiveComponent.SetCollisionEnabled` _sword "PhysicsOnly")
  (`SceneComponent.K2_DetachFromComponent` _sword "KeepRelative" "KeepRelative" "KeepRelative" true)
  (`PrimitiveComponent.SetSimulatePhysics` _sword true))

(event `/Game/_ShadowStrike/Blueprints/BPI_Character.ToggleTargetIndicator`
  (params (`Show?` :type Boolean))
  (bind _targetindicator (`self.TargetIndicator`))
  ;[1 1 1] Toggle Target indicator of enemies
  (if `Show?`
    (`SceneComponent.SetVisibility` _targetindicator true false)
    (else
      (`SceneComponent.SetVisibility` _targetindicator false false))))

(event `/Game/_ShadowStrike/Blueprints/BPI_Character.SetDeadState`
  (params (`Died?` :type Boolean))
  ;[1 1 1] Enable death state
  (set `self.Died?` `Died?`))

(fn `CanBeTargeted?`
  (returns (`Yes?` :type Boolean))
  (return (not (`self.Died?`))))

(fn `GetBowHandLocation`
  (returns (Location :type "Vector Structure"))
  (return (0.0 0.0 0.0)))

(fn `GetCharacterMesh`
  (returns (Mesh :type "SkeletalMeshComponent Object Reference"))
  (return (`self.Mesh`)))

(fn `isDead?`
  (returns (`Dead?` :type Boolean))
  (return (`self.Died?`)))

(fn `UserConstructionScript`)